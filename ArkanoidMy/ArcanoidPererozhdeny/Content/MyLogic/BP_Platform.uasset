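; BP_Platform is a player-controlled platform that moves horizontally in fixed steps and manages lives in a ball game.
; On BeginPlay it binds to a dispatcher on existing BP_Balls; the handler destroys the reported ball, decrements lives and shows GameEnd_Widget when none remain.
; E spawns a limited number of BP_bonus actors at random TargetPoints, destroying each used point to prevent reuse.
; Q prints the ball count for debugging.
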(event `InputAxis|MoveRight`
  (params (AxisValue :type "Float (single-precision)"))
  (if (< AxisValue 0.0)
    (`self.K2_AddActorWorldOffset` (-50.0 0.0 0.0))))

(event `InputAxis|MoveRight`
  (params (AxisValue :type "Float (single-precision)"))
  (if (> AxisValue 0.0)
    (`self.K2_AddActorWorldOffset` (50.0 0.0 0.0))))

(event `Key|Q`
  (params (Key :type "Key Structure"))
  (:`Pressed`
    (bind _outactors (`GameplayStatics.GetAllActorsOfClass` "/Game/MyLogic/BP_Ball.BP_Ball_C"))
    (`KismetSystemLibrary.PrintString` (`KismetStringLibrary.Conv_IntToString` (`KismetArrayLibrary.Array_Length` _outactors)))))

(event `Key|E`
  (params (Key :type "Key Structure"))
  (:`Pressed`
    (if (< (`self.count`) 3)
      (`/Engine/EditorBlueprintResources/StandardMacros.IncrementInt` (`self.count`)
        (:`  `
          (bind _outactors (`GameplayStatics.GetAllActorsOfClass` "/Script/Engine.TargetPoint"))
          (bind _output_get (set `self.targetPoints` (`KismetArrayLibrary.Array_Random` _outactors)))
          (`|SpawnActorFromClass` "/Game/MyLogic/BP_bonus.BP_bonus_C" (`self.GetTransform` _output_get) "Undefined" "MultiplyWithRoot" null null)
          (`KismetSystemLibrary.PrintString` "Destroyed" false false)
          (`KismetSystemLibrary.PrintString` (`KismetSystemLibrary.GetDisplayName` _output_get) false false)
          (`self.K2_DestroyActor` _output_get)
          (bind _outactors_2 (`GameplayStatics.GetAllActorsOfClass` "/Script/Engine.TargetPoint"))
          (`KismetSystemLibrary.PrintString` "exist:" false false)
          (for _index (range (`KismetArrayLibrary.Array_Length` _outactors_2))
            (`KismetSystemLibrary.PrintString` (`KismetSystemLibrary.GetDisplayName` (`|GetArrayItem` _outactors_2 _index)) false false)))))))

(event `self.ReceiveBeginPlay`
  (bind _outactors (`GameplayStatics.GetAllActorsOfClass` "/Game/MyLogic/BP_Ball.BP_Ball_C"))
  (add `/Game/MyLogic/BP_Ball.ToFuncSubstract` _outactors (delegate `substructLife`)))

(event `substructLife`
  (params (which_ball :type "/Game/MyLogic/BP_Ball Object Reference"))
  (`KismetSystemLibrary.PrintString` "Trigger Volume")
  (bind _outactors (`GameplayStatics.GetAllActorsOfClass` "/Game/MyLogic/BP_Ball.BP_Ball_C"))
  (`self.K2_DestroyActor` which_ball)
  (if (> (`KismetArrayLibrary.Array_Length` _outactors) 0)
    (bind _result (`/Engine/EditorBlueprintResources/StandardMacros.DecrementInt` (`self.Lifes`))
      (:`  `
        (if (not (> _result 0))
          (bind _returnvalue (`|CreateWidget` "/Game/MyLogic/GameEnd_Widget.GameEnd_Widget_C"))
          (`UserWidget.AddToViewport` _returnvalue 0))))))

(fn `UserConstructionScript`)