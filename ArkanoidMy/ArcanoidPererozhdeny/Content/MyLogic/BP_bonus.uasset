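; BP_bonus is a bonus actor that adds an extra ball when a BP_Ball overlaps it, then destroys itself.
; The overlap is gated by the FirstBall flag and, after a zero-length Delay, calls DoubleBalls to spawn a BP_Ball offset along Y from the first BP_Platform found.
; BeginPlay prints the bonus actor count; code rotating the new ball's Direction is disconnected.
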(event `self.ReceiveBeginPlay`
  (bind _outactors (`GameplayStatics.GetAllActorsOfClass` "BP_bonus_C"))
  (`KismetSystemLibrary.PrintString` (`KismetStringLibrary.Conv_IntToString` (`KismetArrayLibrary.Array_Length` _outactors))))

(event `self.ReceiveActorBeginOverlap`
  (params (OtherActor :type "Actor Object Reference"))
  (bind _asbp_ball (cast `/Game/MyLogic/BP_Ball` OtherActor))
  (if (`self.FirstBall`)
    (bind _outactors (`GameplayStatics.GetAllActorsOfClass` "/Game/MyLogic/BP_Platform.BP_Platform_C"))
    (set `self.FirstBall` false)
    (`KismetSystemLibrary.Delay` 0.0)
    (bind _returnvalue (`self.GetTransform` (`|GetArrayItem` _outactors)))
    (`self.Double Balls` (`KismetMathLibrary.Conv_VectorToTransform` (`KismetMathLibrary.MakeVector` (.x (.location _returnvalue)) (+ (.y (.location _returnvalue)) -100.0) (.z (.location _returnvalue)))))
    (`self.K2_DestroyActor`)))

(fn `Double Balls`
  (params (BallTransform :type "Transform Structure (by ref)"))
  (bind _returnvalue (`|SpawnActorFromClass` "/Game/MyLogic/BP_Ball.BP_Ball_C" BallTransform "Undefined" "MultiplyWithRoot" null null)))

(fn `UserConstructionScript`)