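; BP_Ball is a bouncing ball actor that moves itself along a direction at a set speed.
; Each Tick it does a swept world offset, and on a blocking hit reflects its direction off the hit normal flattened onto the horizontal plane.
; Overlapping a TriggerVolume prints a debug string and calls CallToFuncSubstract.
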(event `self.ReceiveTick`
  (params (DeltaSeconds :type "Float (single-precision)"))
  (bind _sweephitresult (`self.K2_AddActorWorldOffset` (* (* (`self.Direction`) (`self.Speed`)) DeltaSeconds) true))
  (bind (_bblockinghit _binitialoverlap _time _distance _location _impactpoint _normal) (`GameplayStatics.BreakHitResult` _sweephitresult))
  (if _bblockinghit
    (`KismetSystemLibrary.PrintString` (`KismetStringLibrary.Conv_VectorToString` _normal) false false)
    (set `self.Direction` (`KismetMathLibrary.GetReflectionVector` (`self.Direction`) (`KismetMathLibrary.ProjectVectorOnToPlane` _normal (0.0 0.0 1.0))))))

(event `self.ReceiveActorBeginOverlap`
  (params (OtherActor :type "Actor Object Reference"))
  (cast `TriggerVolume` OtherActor)
  (`KismetSystemLibrary.PrintString` "YEsS")
  (`self.ToFuncSubstract` self))

(fn `UserConstructionScript`)